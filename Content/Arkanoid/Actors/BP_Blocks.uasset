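; BP_Blocks is an Arkanoid brick grid actor that spawns breakable blocks and awards points when they are hit.
; Its construction script adds a BP_LifesBlocks component at each cell of a grid sized by X and Y and spaced by Pading.
; On hit, it damages the struck block component and sends PointsRewardOnHit to the player pawn's points display.
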(event Collision|EventHit
  (params (MyComp :type Primitive%20Component%20Object%20Reference) (Other :type Actor%20Object%20Reference) (OtherComp :type Primitive%20Component%20Object%20Reference) (bSelfMoved :type Boolean) (HitLocation :type Vector :default "0, 0, 0") (HitNormal :type Vector :default "0, 0, 0") (NormalImpulse :type Vector :default "0, 0, 0") (Hit :type Hit%20Result%20Structure%20%28by%20ref%29))
  (bind _asbp_lifes_blocks (Utilities|Casting|CastToBP_LifesBlocks MyComp))
  (Default|Damage _asbp_lifes_blocks)
  (Class|BPPlayerInterface|UpdateCurrentPoints(Message) (Game|Player|GetPlayerPawn 0) (Variables|Default|GetPoints%20Reward%20On%20Hit)))

(fn ConstructionScript
  (bind _pading (Variables|Default|GetPading))
  (for _index (range 0 (Variables|Default|GetX))
    (for _index_2 (range 0 (Variables|Default|GetY))
      (AddComponent|AddBPLifesBlocks false (Math|Transform|MakeTransform (Math|Vector|MakeVector (Math|Conversions|ToFloat(Integer) (* _index _pading)) (Math|Conversions|ToFloat(Integer) (* _index_2 _pading)) 0.0)) 0))))