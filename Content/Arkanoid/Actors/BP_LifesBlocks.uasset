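; BP_LifesBlocks is a multi-hit block component for the Arkanoid game that can drop a bonus when destroyed.
; Each Damage call decrements its life counter and swaps the material while lives remain.
; When lives reach zero, it destroys itself and calls SpawnBonus, which has an even chance of spawning a BP_Bonus of a randomly selected type at the block's location.
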(event EventBeginPlay)

(event EventTick
  (params (DeltaSeconds :type Float%20%28single-precision%29)))

(fn Damage
  (bind _result (Math|Integer|DecrementInt (Variables|Default|GetLifes))
    (:%20%20
      (if (== _result 0)
        (Components|DestroyComponent)
        (CallFunction|SpawnBonus)
        (else
          (Rendering|Material|SetMaterial 0 "/AnimationSharing/AnimSharingGreen.AnimSharingGreen"))))))

(fn SpawnBonus
  (if (Math|Random|RandomBoolwithWeight 0.5)
    (Game|SpawnActorfromClass "/Game/Arkanoid/Actors/BP_Bonus.BP_Bonus_C" (Math|Transform|MakeTransform (Transformation|GetWorldLocation) "0, 0, 0" "1,1,1") "AlwaysSpawn" 0 (Utilities|Select :Index (Math|Random|RandomIntegerinRange 0 4) :Option%200 "NewEnumerator0" :Option%201 "NewEnumerator2" :Option%202 "NewEnumerator3" :Option%203 "NewEnumerator4" :Option%204 "NewEnumerator7") 0)
    (return)))