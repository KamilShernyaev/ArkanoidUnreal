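; BP_Bonus is an Arkanoid pickup that falls along negative X and grants its BonusType effect when it overlaps the player's pawn.
; Tick moves it by a swept world offset scaled by Speed, and overlapping a KillZVolume destroys it.
; Pawn effects and ball spawning call BP_Pawn, while Fast Ball affects only the BP_Ball returned by GetActorOfClass.
; The construction script picks the cube's material from BonusType.
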(event EventTick
  (params (DeltaSeconds :type Float%20%28single-precision%29))
  (Transformation|AddActorWorldOffset (* (* "-100.000000,0.000000, 0" (Variables|Default|GetSpeed)) DeltaSeconds) true))

(event Collision|EventActorBeginOverlap
  (params (OtherActor :type Actor%20Object%20Reference))
  (Utilities|FlowControl|Sequence
    (:then_0
      (Utilities|Casting|CastToKillZVolume OtherActor)
      (Actor|DestroyActor))
    (:then_1
      (bind _asbp_pawn (Utilities|Casting|CastToBP_Pawn OtherActor))
      (Actor|DestroyActor)
      (switch Utilities|FlowControl|Switch|SwitchonE_Bonuses (Variables|Default|GetBonus%20Type)
        (:NewEnumerator0
          (Default|SpawnBall _asbp_pawn))
        (:NewEnumerator2
          (bind _returnvalue (Actor|GetActorOfClass "/Game/Arkanoid/Actors/BP_Ball.BP_Ball_C"))
          (Default|FastBall _returnvalue))
        (:NewEnumerator3
          (Default|BigPawn _asbp_pawn))
        (:NewEnumerator4
          (Default|SmallPawn _asbp_pawn))
        (:NewEnumerator7
          (Default|FastPawn _asbp_pawn))))))

(fn ConstructionScript
  (Rendering|Material|SetMaterial (Variables|Default|GetCube) 0 (Utilities|Select :Index (Variables|Default|GetBonus%20Type) :NewEnumerator0 "/DatasmithContent/Materials/AliasMaster.AliasMaster" :NewEnumerator2 "/Engine/VREditor/BasicMeshes/MI_Cube_01.MI_Cube_01" :NewEnumerator3 "/AnimationSharing/AnimSharingGreen.AnimSharingGreen" :NewEnumerator4 "/AnimationSharing/AnimSharingBlue.AnimSharingBlue" :NewEnumerator7 "/Engine/EngineDebugMaterials/ShadedLevelColorationLitMaterial.ShadedLevelColorationLitMaterial")))