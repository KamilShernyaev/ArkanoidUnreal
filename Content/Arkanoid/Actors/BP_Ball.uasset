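; BP_Ball is the Arkanoid ball, moved every Tick by a swept offset along its Direction and Speed.
; Blocking hits reflect Direction, zeroing any Z in the normal to keep bounces planar.
; FastBall raises speed, turns the sphere red and starts a short timer, while NormalSpeed restores speed and material.
; Overlapping a KillZVolume deducts player points, calls OnDead, removes the ball from BP_GameMode and destroys it.
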(event EventTick
  (params (DeltaSeconds :type Float%20%28single-precision%29))
  (bind _sweephitresult (Transformation|AddActorWorldOffset (* (* (Variables|Default|GetDirection) (Variables|Default|GetSpeed)) DeltaSeconds) true))
  (if (.bBlockingHit (Collision|BreakHitResult _sweephitresult))
    (if (!= (.Z (Math|Vector|BreakVector (.Normal (Collision|BreakHitResult _sweephitresult)))) 0.0)
      (Variables|Default|SetDirection (Math|Vector|GetReflectionVector (Variables|Default|GetDirection) (Math|Vector|MakeVector (.X (Math|Vector|BreakVector (.Normal (Collision|BreakHitResult _sweephitresult)))) (.Y (Math|Vector|BreakVector (.Normal (Collision|BreakHitResult _sweephitresult)))) 0.0)))
      (else
        (Variables|Default|SetDirection (Math|Vector|GetReflectionVector (Variables|Default|GetDirection) (.Normal (Collision|BreakHitResult _sweephitresult))))))))

(event Collision|EventActorBeginOverlap
  (params (OtherActor :type Actor%20Object%20Reference))
  (Utilities|Casting|CastToKillZVolume OtherActor)
  (Class|BPPlayerInterface|MinusCurrentPoints(Message) (Game|Player|GetPlayerPawn 0) (Variables|Default|GetMinusPoint))
  (Default|CallOnDead)
  (bind _asbp_game_mode (Utilities|Casting|CastToBP_GameMode (Game|GetGameMode)))
  (Default|RemoveBall _asbp_game_mode self)
  (Actor|DestroyActor))

(fn ConstructionScript)

(fn FastBall
  (Variables|Default|SetSpeed 2e+01)
  (Utilities|Time|SetTimerbyEvent (EventDispatchers|CreateEvent :!event NormalSpeed) 3.0)
  (Rendering|Material|SetMaterial (Variables|Default|GetSphere) 0 "/AnimationSharing/AnimSharingRed.AnimSharingRed")
  (return))

(fn NormalSpeed
  (Variables|Default|SetSpeed 1e+01)
  (Rendering|Material|SetMaterial (Variables|Default|GetSphere) 0 "/Engine/BasicShapes/BasicShapeMaterial.BasicShapeMaterial")
  (return))