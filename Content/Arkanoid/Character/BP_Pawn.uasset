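; Player paddle pawn for an Arkanoid game, moved sideways with swept offsets and keeping the score.
; BeginPlay shows the HUD, then after a delay spawns a ball, registers it with BP_GameMode and binds its death event.
; Small, Big and Fast functions change scale or speed plus material and start timers, while NormalPawn restores defaults.
; TryCreateBall spawns another ball when the game mode's count equals one.
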(event EventUpdateCurrentPoints
  (params (Points%20Delta :type Integer))
  (Variables|Default|SetCurrentPoints (+ Points%20Delta (Variables|Default|GetCurrentPoints))))

(event EventMinusCurrentPoints
  (params (PointsMinus :type Integer))
  (Variables|Default|SetCurrentPoints (- (Variables|Default|GetCurrentPoints) PointsMinus)))

(event EventBeginPlay
  (bind _returnvalue (UserInterface|CreateWidget "/Game/Arkanoid/HUD/BP_PlayerHUD.BP_PlayerHUD_C"))
  (UserInterface|Viewport|AddtoViewport _returnvalue 0)
  (Utilities|FlowControl|Delay 3.0)
  (CallFunction|SpawnBall))

(event Input|AxisEvents|InputAxisMoveRight
  (params (AxisValue :type Float%20%28single-precision%29))
  (if (!= AxisValue 0.0)
    (Transformation|AddActorWorldOffset (Math|Vector|MakeVector 0.0 (* (Variables|Default|GetSpeedPawn) (Utilities|Time|GetWorldDeltaSeconds) AxisValue) 0.0) true)))

(fn ConstructionScript)

(fn SpawnBall
  (bind _returnvalue (Game|SpawnActorfromClass "/Game/Arkanoid/Actors/BP_Ball.BP_Ball_C" (Math|Conversions|ToTransform(Vector) (Transformation|GetWorldLocation (Variables|Default|GetCapsule))) "Undefined" 0 0))
  (bind _output_get (Variables|Default|SetPlayingBall _returnvalue))
  (bind _asbp_game_mode (Utilities|Casting|CastToBP_GameMode (Game|GetGameMode)))
  (Default|AddBall _asbp_game_mode _output_get)
  (EventDispatchers|BindEventtoOnDead _output_get (EventDispatchers|CreateEvent :!event TryCreateBall))
  (return))

(fn TryCreateBall
  (bind _asbp_game_mode (Utilities|Casting|CastToBP_GameMode (Game|GetGameMode)))
  (if (== (Default|GetCountOfBalls _asbp_game_mode) 1)
    (CallFunction|SpawnBall)))

(fn SmallPawn
  (bind _cube (Variables|Default|GetCube))
  (Transformation|SetWorldTransform _cube (Math|Transform|MakeTransform (Transformation|GetWorldLocation _cube) (Transformation|GetWorldRotation _cube) "1.500000,-0.250000,0.800000") false false)
  (Utilities|Time|SetTimerbyEvent (EventDispatchers|CreateEvent :!event NormalPawn) 3.0)
  (Rendering|Material|SetMaterial (Variables|Default|GetCube) 0 "/AnimationSharing/AnimSharingBlue.AnimSharingBlue")
  (return))

(fn NormalPawn
  (bind _cube (Variables|Default|GetCube))
  (Transformation|SetWorldTransform _cube (Math|Transform|MakeTransform (Transformation|GetWorldLocation _cube) (Transformation|GetWorldRotation _cube) "2.500000,-0.250000,0.800000") false false)
  (Variables|Default|SetSpeedPawn 4e+03)
  (Rendering|Material|SetMaterial (Variables|Default|GetCube) 0 "/Engine/EditorMeshes/ColorCalibrator/M_ClearCoat.M_ClearCoat")
  (return))

(fn BigPawn
  (bind _cube (Variables|Default|GetCube))
  (Transformation|SetWorldTransform _cube (Math|Transform|MakeTransform (Transformation|GetWorldLocation _cube) (Transformation|GetWorldRotation _cube) "5.000000,-0.250000,0.800000") false false)
  (Utilities|Time|SetTimerbyEvent (EventDispatchers|CreateEvent :!event NormalPawn) 8.0)
  (Rendering|Material|SetMaterial (Variables|Default|GetCube) 0 "/AnimationSharing/AnimSharingGreen.AnimSharingGreen")
  (return))

(fn FastPawn
  (Variables|Default|SetSpeedPawn 8e+03)
  (Utilities|Time|SetTimerbyEvent (EventDispatchers|CreateEvent :!event NormalPawn) 5.0)
  (Rendering|Material|SetMaterial (Variables|Default|GetCube) 0 "/Engine/EngineDebugMaterials/ShadedLevelColorationLitMaterial.ShadedLevelColorationLitMaterial")
  (return))

(fn StartGame)

(fn GetCurrentPoints
  (return (Variables|Default|GetCurrentPoints)))